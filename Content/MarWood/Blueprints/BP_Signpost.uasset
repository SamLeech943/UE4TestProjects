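; BP_Signpost is an interactable signpost that shows its text in a Dialogue_UI widget on screen.
; Interact toggles the window: it removes an existing widget and clears the reference, or creates one for player controller 0 and fills it with the Text variable.
; A component end-overlap event also removes the widget, without clearing the stored reference.
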(event OnComponentEndOverlap()
  (params (OverlappedComponent :type Primitive%20Component%20Object%20Reference) (OtherActor :type Actor%20Object%20Reference) (OtherComp :type Primitive%20Component%20Object%20Reference) (OtherBodyIndex :type Integer))
  (Widget|RemovefromParent (Variables|Default|GetDialogue%20Window)))

(event EventBeginPlay)

(event Collision|EventActorBeginOverlap
  (params (OtherActor :type Actor%20Object%20Reference)))

(event EventTick
  (params (DeltaSeconds :type Float%20%28single-precision%29)))

(event EventInteract
  (Utilities|IsValid (Variables|Default|GetDialogue%20Window)
    (:Is%20Valid
      (Widget|RemovefromParent (Variables|Default|GetDialogue%20Window))
      (Variables|Default|SetDialogue%20Window 0))
    (:Is%20Not%20Valid
      (bind _returnvalue (UserInterface|CreateWidget "/Game/MarWood/UI/Dialogue_UI.Dialogue_UI_C" (Game|GetPlayerController 0)))
      (bind _output_get (Variables|Default|SetDialogue%20Window _returnvalue))
      (UserInterface|Viewport|AddtoViewport _output_get 0)
      (Variables|/Game/MarWood/UI/Dialogue_UI.Dialogue_UI_C|SetDialogueText (Variables|Default|GetDialogue%20Window) (Variables|Default|GetText)))))

(fn ConstructionScript)