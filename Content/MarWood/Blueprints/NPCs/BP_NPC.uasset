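; BP_NPC is an interactable NPC that shows data-table dialogue to the player line by line.
; On BeginPlay it caches the Dialogue table rows matching its NPCID.
; Each Interact advances LineCurrent and creates or updates a Dialogue_UI widget with the row matching ConversationID and that line.
; The window is removed when an overlap with its Box ends, or, with a line reset, when the lookup does not find exactly one match.
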(event OnComponentEndOverlap(Box)
  (params (OverlappedComponent :type Primitive%20Component%20Object%20Reference) (OtherActor :type Actor%20Object%20Reference) (OtherComp :type Primitive%20Component%20Object%20Reference) (OtherBodyIndex :type Integer))
  ;[1 1 1] Remove Dilogue Window if player leaves the area
  (Widget|RemovefromParent (Variables|Default|GetDialogueWindow)))

(event Collision|EventActorBeginOverlap
  (params (OtherActor :type Actor%20Object%20Reference)))

(event EventTick
  (params (DeltaSeconds :type Float%20%28single-precision%29)))

(event EventBeginPlay
  ;[1 1 1] Search for Dialogue usin the data table
  (bind _outrownames (DataTable|GetDataTableRowNames "/Game/MarWood/Data/Dialogue.Dialogue"))
  (for _array_element _outrownames
    (bind _returnvalue (Utilities|GetDataTableRow "/Game/MarWood/Data/Dialogue.Dialogue" _array_element)
      (:then
        (if (== (.NPC_ID (Utilities|Struct|BreakDialogue_Struct _returnvalue)) (Variables|Default|GetNPC_ID))
          (Utilities|Array|Add (Variables|Default|GetDialogue) _array_element))))))

(event EventInteract
  ;[1 1 1] Adds Diologue
  (Math|Integer|IncrementInt (Variables|Default|GetLineCurrent)
    (:%20%20
      (CallFunction|DialogueCreate))))

(fn ConstructionScript)

(fn DialogueCreate
  (Utilities|IsValid (Variables|Default|GetDialogueWindow)
    (:Is%20Valid
      (bind _returned_line (CallFunction|DialogueGetLine))
      (Variables|/Game/MarWood/UI/Dialogue_UI.Dialogue_UI_C|SetDialogueText (Variables|Default|GetDialogueWindow) _returned_line))
    (:Is%20Not%20Valid
      (bind _returnvalue (UserInterface|CreateWidget "/Game/MarWood/UI/Dialogue_UI.Dialogue_UI_C" (Game|GetPlayerController 0)))
      (bind _output_get (Variables|Default|SetDialogueWindow _returnvalue))
      (UserInterface|Viewport|AddtoViewport _output_get 0)
      (bind _returned_line_2 (CallFunction|DialogueGetLine))
      (Variables|/Game/MarWood/UI/Dialogue_UI.Dialogue_UI_C|SetDialogueText (Variables|Default|GetDialogueWindow) _returned_line_2))))

(fn DialogueGetLine
  (for _array_element (Variables|Default|GetDialogue)
    (bind _returnvalue (Utilities|GetDataTableRow "/Game/MarWood/Data/Dialogue.Dialogue" _array_element)
      (:then
        (if (and (== (.Conversation_ID (Utilities|Struct|BreakDialogue_Struct _returnvalue)) (Variables|Default|GetConversation_ID)) (== (.Line_ID (Utilities|Struct|BreakDialogue_Struct _returnvalue)) (Variables|Default|GetLineCurrent)))
          (Utilities|Array|Add (LocalVariables|GetReturnedLines) (.Dialogue (Utilities|Struct|BreakDialogue_Struct _returnvalue)))))))
  (if (== (Utilities|Array|Length (LocalVariables|GetReturnedLines)) 1)
    (return (Utilities|Array|Get(acopy) (LocalVariables|GetReturnedLines)))
    (else
      (Widget|RemovefromParent (Variables|Default|GetDialogueWindow))
      (Variables|Default|SetDialogueWindow 0)
      (Variables|Default|SetLineCurrent 0))))